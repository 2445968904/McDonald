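; Demo actor that connects to a MySQL database and tests queries through UMG widgets.
; BeginPlay shows a login widget; a successful connection opens the basic query demo for select, single or batch update, and close.
; Widget events call the inherited connection and query functions, whose status callbacks relay results and errors back to the widgets.
; An image query demo is also wired, but its widget creation is disconnected and never runs.
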(event Custom|LoginToServer_Event
  (params (Server :type String) (DataBase :type String) (UserID :type String) (Password :type String) (Port :type Integer))
  ;[0 0.163 1] Create DBConnection Widget
  (Class|MySQLDBConnectionActor|CreateNewConnection Server DataBase UserID Password Port))

(event Custom|OnCallUpdateQuery
  (params (UpdateQuery :type String))
  ;[1 1 1] Simple Query Execution
  ;;[0 0.2 0.54] This is Basic Query Demo. Plug this in to test out storing and retrieving data from Database
  ;;;[1 1 1] "Update Data from Query" is used to Insert Data into the Table which was already created. If the table does not exist, it will throw exception which will be returned in the Error message output
  (Class|MySQLDBConnectionActor|UpdateDatafromQuery (Variables|Default|GetConnection%20ID) UpdateQuery))

(event Custom|OnCallUpdateImageFromPath
  (params (Query :type String) (UpdateParameter :type String) (ParameterID :type Integer) (ImagePath :type String))
  ;[1 1 1] Image Query Execution
  ;;[0 0.2 0.54] This is Image Query Demo. Use this to test inserting and selecting image from your database
  (Class|MySQLDBConnectionActor|UpdateImagefromPath (Variables|Default|GetConnection%20ID) Query UpdateParameter ParameterID ImagePath))

(event Custom|OnCallSelectImageFromQuery
  (params (Query :type String))
  ;[1 1 1] Image Query Execution
  ;;[0 0.2 0.54] This is Image Query Demo. Use this to test inserting and selecting image from your database
  (Class|MySQLDBConnectionActor|SelectImagefromQuery (Variables|Default|GetConnection%20ID) Query))

(event Custom|OnCallUpdateImageQuery
  (params (UpdateQuery :type String))
  ;[1 1 1] Image Query Execution
  ;;[0 0.2 0.54] This is Image Query Demo. Use this to test inserting and selecting image from your database
  (Class|MySQLDBConnectionActor|UpdateDatafromQuery (Variables|Default|GetConnection%20ID) UpdateQuery))

(event Custom|OnCallSelectQuery
  (params (Query :type String))
  ;[1 1 1] Simple Query Execution
  ;;[0 0.2 0.54] This is Basic Query Demo. Plug this in to test out storing and retrieving data from Database
  ;;;[1 1 1] "Select Data from Query" takes your Select Query as string input, and result the result in two different formats, columnwise and rowwise
  (Class|MySQLDBConnectionActor|SelectDatafromQuery (Variables|Default|GetConnection%20ID) Query))

(event Custom|OnCloseConnection
  ;[1 1 1] Simple Query Execution
  ;;[0 0.2 0.54] This is Basic Query Demo. Plug this in to test out storing and retrieving data from Database
  ;;;[1 1 1] Close Connection
  (Class|MySQLDBConnectionActor|CloseConnection (Variables|Default|GetConnection%20ID))
  (Default|OnConnectionClosed (Variables|Default|GetDBConnectionWidget)))

(event Custom|OnUpdateMultipleQueries
  (params (UpdateQueries :type Array%20of%20Strings))
  ;[1 1 1] Simple Query Execution
  ;;[0 0.2 0.54] This is Basic Query Demo. Plug this in to test out storing and retrieving data from Database
  ;;;[1 1 1] Update Multiple Queries at Once
  (Class|MySQLDBConnectionActor|UpdateDatafromMultipleQueries (Variables|Default|GetConnection%20ID) UpdateQueries))

(event EventBeginPlay
  (bind _returnvalue (Game|GetPlayerController 0))
  (Variables|/Script/Engine.PlayerController|SetbShowMouseCursor _returnvalue true)
  (Input|SetInputModeUIOnly _returnvalue 0 "DoNotLock" false)
  ;[0 0.163 1] Create DBConnection Widget
  (bind _returnvalue_2 (UserInterface|CreateWidget "/Game/Widgets/UMG_DBConnection.UMG_DBConnection_C"))
  (bind _output_get (Variables|Default|SetDBConnectionWidget _returnvalue_2))
  (UserInterface|Viewport|AddtoViewport _output_get 0)
  (EventDispatchers|AssignLogintoServer (Variables|Default|GetDBConnectionWidget) (delegate Custom|LoginToServer_Event)))

(event EventOnConnectionStateChanged
  (params (ConnectionStatus :type Boolean) (ConnectionID :type Integer) (ErrorMessage :type String))
  ;[1 0.2151 0.2118] On ConnectionStateChanged
  (Variables|Default|SetConnection%20ID ConnectionID)
  (Default|OnConnectionStateUpdated (Variables|Default|GetDBConnectionWidget) ConnectionStatus ErrorMessage)
  (if ConnectionStatus
    ;[1 1 1] Simple Query Execution
    ;;[0 0.2 0.54] This is Basic Query Demo. Plug this in to test out storing and retrieving data from Database
    (bind _returnvalue (UserInterface|CreateWidget "/Game/Widgets/UMG_BasicQueryDemo.UMG_BasicQueryDemo_C"))
    (bind _output_get (Variables|Default|SetMySQLQueryWidget _returnvalue))
    (UserInterface|Viewport|AddtoViewport _output_get 0)
    (EventDispatchers|AssignOnCallUpdateQuery (Variables|Default|GetMySQLQueryWidget) (delegate Custom|OnCallUpdateQuery))
    (EventDispatchers|AssignOnCallSelectQuery (Variables|Default|GetMySQLQueryWidget) (delegate Custom|OnCallSelectQuery))
    (EventDispatchers|BindEventtoOnCallUpdateMultipleQueries (Variables|Default|GetMySQLQueryWidget) (delegate Custom|OnUpdateMultipleQueries))
    (EventDispatchers|BindEventtoOnCloseConnection (Variables|Default|GetMySQLQueryWidget) (delegate Custom|OnCloseConnection))))

(event EventOnQueryUpdateStatusChanged
  (params (ConnectionID :type Integer) (QueryID :type Integer) (IsSuccessful :type Boolean) (ErrorMessage :type String))
  ;[1 1 1] Simple Query Execution
  ;;[1 1 1] On Query Update Status Changed
  (Variables|Default|SetCurrentQueryID QueryID)
  (Utilities|FlowControl|Sequence
    (:then_0
      (Utilities|IsValid (Variables|Default|GetMySQLQueryWidget)
        (:Is%20Valid
          (Default|OnExecutionStatusChanged (Variables|Default|GetMySQLQueryWidget) IsSuccessful ErrorMessage (Variables|Default|GetCurrentQueryID)))))
    (:then_1
      (Utilities|IsValid (Variables|Default|GetMySQLImageQueryWidget)
        (:Is%20Valid
          (Default|OnExecutionStatusChanged (Variables|Default|GetMySQLImageQueryWidget) IsSuccessful ErrorMessage))))))

(event EventOnImageUpdateStatusChanged
  (params (ConnectionID :type Integer) (QueryID :type Integer) (IsSuccessful :type Boolean) (ErrorMessage :type String))
  ;[1 1 1] Image Query Execution
  ;;[1 1 1] On Image Update Status Changed
  (Default|OnExecutionStatusChanged (Variables|Default|GetMySQLImageQueryWidget) IsSuccessful ErrorMessage))

(event EventOnImageSelectStatusChanged
  (params (ConnectionID :type Integer) (QueryID :type Integer) (IsSuccessful :type Boolean) (ErrorMessage :type String) (SelectedTexture :type Texture%202D%20Object%20Reference))
  ;[1 1 1] Image Query Execution
  ;;[1 1 1] On Image Select Status Changed
  (Default|OnExecutionStatusChanged (Variables|Default|GetMySQLImageQueryWidget) IsSuccessful ErrorMessage)
  (Default|OnImageReceived (Variables|Default|GetMySQLImageQueryWidget) SelectedTexture))

(event EventOnQuerySelectStatusChanged
  (params (ConnectionID :type Integer) (QueryID :type Integer) (IsSuccessful :type Boolean) (ErrorMessage :type String) (ResultByColumn :type Array%20of%20My%20SQL%20Data%20Table%20Structures) (ResultByRow :type Array%20of%20My%20SQL%20Data%20Row%20Structures))
  ;[1 1 1] Simple Query Execution
  ;;[1 1 1] On Query Select Status Changed
  (Variables|Default|SetCurrentQueryID QueryID)
  (Utilities|IsValid (Variables|Default|GetMySQLQueryWidget)
    (:Is%20Valid
      (Default|OnSelectionStatusChanges (Variables|Default|GetMySQLQueryWidget) IsSuccessful ErrorMessage (Variables|Default|GetCurrentQueryID) ResultByColumn ResultByRow))))

(fn ConstructionScript)