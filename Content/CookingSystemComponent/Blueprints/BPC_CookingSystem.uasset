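; Player component that runs an Overcooked-style cooking loop: carrying, combining and chopping ingredients, and delivering orders.
; InteractEvent sphere-traces ahead, casting the hit to dispenser, delivery station, trash bin or desk to move held items.
; With SimulateGame on, Tick-driven Delay macros add random DataTable orders increasingly often and count down timers, pausing into a lose screen past FatalNumber.
; Tick also drives gated chopping; plates matching orders' ingredients earn money, and order changes rebuild the HUD.
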(event Custom|InitSystem
  (params (PlayerRef :type BP%20Character%20Object%20Reference) (IngredientSocket :type Scene%20Component%20Object%20Reference) (SimulateGame? :type Boolean))
  ;[1 0 0.04868] Init Component
  (Variables|Default|SetPlayerRef PlayerRef)
  (Variables|Default|SetIngredientSocket IngredientSocket)
  (Variables|Default|SetSimulateGame? SimulateGame?)
  (bind _returnvalue (UserInterface|CreateWidget "/Game/CookingSystemComponent/Widgets/WB_HUD.WB_HUD_C" 0 self))
  (bind _output_get (Variables|Default|SetHUDRef _returnvalue))
  (UserInterface|Viewport|AddtoViewport _output_get 0))

(event Custom|InteractEvent
  ;[0 0.7401 1] Interact
  (bind (_hit _hitactor) (CallFunction|SphereTracebyChanel))
  (if _hit
    ;[0 0 1] Dispatch Ingredient
    (bind _asbp_ingredient_dispatcher (Utilities|Casting|CastToBP_IngredientDispatcher _hitactor)
      (:then
        (CallFunction|DispatcherFunction _asbp_ingredient_dispatcher))
      (:CastFailed
        ;[1 1 0] Deliver Order
        (bind _asbp_delivery_station (Utilities|Casting|CastToBP_DeliveryStation _hitactor)
          (:then
            (CallFunction|DeliveryStationFunction _asbp_delivery_station))
          (:CastFailed
            ;[0 1 0.8739] Trash Bin
            (bind _asbp_trash_bin (Utilities|Casting|CastToBP_TrashBin _hitactor)
              (:then
                (CallFunction|TrashBinFunction _asbp_trash_bin))
              (:CastFailed
                ;[1 0 0] PickUp/Drop
                (bind _asbp_kitchen_desk (Utilities|Casting|CastToBP_KitchenDesk _hitactor))
                (CallFunction|KitchenDeskFunction _asbp_kitchen_desk)))))))))

(event Custom|ChopEvent
  ;[0 1 0] Chop
  (Utilities|ChopFunction) ; enters at Open
)

(event EventBeginPlay
  (bind _datatable (Variables|Default|GetDataTable))
  (bind _outrownames (DataTable|GetDataTableRowNames _datatable))
  (for _array_element _outrownames
    (bind _returnvalue (Utilities|GetDataTableRow _datatable _array_element)
      (:then
        (Utilities|Array|Add (Variables|Default|GetOrderAll) _returnvalue))))
  (bind _returnvalue_2 (Actor|GetActorOfClass "/Game/CookingSystemComponent/Blueprints/ValueUpdate.ValueUpdate_C"))
  (Variables|Default|SetFatalNumber (Variables|/Game/CookingSystemComponent/Blueprints/ValueUpdate.ValueUpdate_C|GetFatalNumber _returnvalue_2)))

(event EventTick
  (params (DeltaSeconds :type Float%20%28single-precision%29))
  ;[0 1 0.2801] Tick
  (Utilities|FlowControl|Sequence
    (:then_0
      ;[0 1 0] Chop
      (Utilities|ChopFunction))
    (:then_1
      ;[1 0 1] Add Order
      (if (Variables|Default|GetSimulateGame?)
        (Utilities|AddOrderFunction)))
    (:then_2
      ;[1 0 0.101] Update Orders
      (if (Variables|Default|GetSimulateGame?)
        (Utilities|UpdateOrdersFunction)))))

(fn SphereTracebyChanel
  (bind _playerref (Variables|Default|GetPlayerRef))
  (bind _movingdirectionarrow (Variables|/Game/CookingSystemComponent/Blueprints/BP_Character.BP_Character_C|GetMovingDirectionArrow _playerref))
  (bind _returnvalue (Transformation|GetWorldLocation _movingdirectionarrow))
  (bind (_outhit _returnvalue_2) (Collision|SphereTraceByChannel _returnvalue (+ _returnvalue (* (Math|Vector|GetForwardVector _movingdirectionarrow) (Variables|TraceSphere|GetReach))) (Variables|TraceSphere|GetRadius) "TraceTypeQuery1" false 0 "None"))
  (return _returnvalue_2 (.HitActor (Collision|BreakHitResult _outhit))))

(fn DispatcherFunction
  (params (IngredientDispatcher :type BP%20Ingredient%20Dispatcher%20Object%20Reference))
  (bind _ingredientsocket (Variables|Default|GetIngredientSocket))
  (Utilities|IsValid (Variables|Ingredient|GetCurrentIngredient)
    (:Is%20Not%20Valid
      (bind _returnvalue (Game|SpawnActorfromClass (Utilities|Select :Index (Variables|/Game/CookingSystemComponent/Blueprints/Furnitures/BP_IngredientDispatcher.BP_IngredientDispatcher_C|GetIngredientToDispatch IngredientDispatcher) :NewEnumerator0 "/Game/CookingSystemComponent/Blueprints/Ingredients/BP_Meat.BP_Meat_C" :NewEnumerator1 "/Game/CookingSystemComponent/Blueprints/Ingredients/BP_GrilledMeat.BP_GrilledMeat_C" :NewEnumerator2 "/Game/CookingSystemComponent/Blueprints/Ingredients/BP_Tomato.BP_Tomato_C" :NewEnumerator3 "/Game/CookingSystemComponent/Blueprints/Ingredients/BP_ChoopedTomato.BP_ChoopedTomato_C" :NewEnumerator4 "/Game/CookingSystemComponent/Blueprints/Ingredients/BP_Lettuce.BP_Lettuce_C" :NewEnumerator5 "/Game/CookingSystemComponent/Blueprints/Ingredients/BP_ChoopedLettuce.BP_ChoopedLettuce_C" :NewEnumerator8 "/Game/CookingSystemComponent/Blueprints/Ingredients/BP_Bread.BP_Bread_C" :NewEnumerator9 "/Game/CookingSystemComponent/Blueprints/Ingredients/BP_Potato.BP_Potato_C") (Transformation|GetSocketTransform _ingredientsocket "None" "RTS_World") "AdjustIfPossibleButAlwaysSpawn" 0 0))
      (bind _output_get (Variables|Ingredient|SetCurrentIngredient _returnvalue))
      (Transformation|AttachComponentToComponent _output_get _ingredientsocket "None" "SnapToTarget" "KeepWorld" "KeepWorld" true)
      (return))))

(fn DeliveryStationFunction
  (params (DeliveryStation :type BP%20Delivery%20Station%20Object%20Reference))
  (bind _orders (Variables|Orders|GetOrders))
  (bind _asbp_plate (Utilities|Casting|CastToBP_Plate (Variables|Ingredient|GetCurrentIngredient))
    (:then
      ;[1 1 1] Deliver Order
      (if (Variables|Default|GetSimulateGame?)
        (bind (_array_element _array_index) (Utilities|Array|ForEachLoopwithBreak _orders :!label _label)
          (:LoopBody
            (bind _bool (CallFunction|Check (Variables|/Game/CookingSystemComponent/Blueprints/Ingredients/BP_Ingredient.BP_Ingredient_C|GetNowHaveFood _asbp_plate) (.Ingredient (Utilities|Struct|BreakST_FoodCompile (.foodcompile _array_element)))))
            (if _bool
              (Variables|Default|SetMoney (+ (Variables|Default|GetMoney) (.Money (Utilities|Struct|BreakST_FoodCompile (.foodcompile _array_element)))))
              (Utilities|Array|RemoveIndex _orders _array_index)
              (Default|Restart _asbp_plate :!label _label_2)
              (Transformation|DetachFromActor (Variables|Ingredient|GetCurrentIngredient) "KeepWorld" "KeepWorld" "KeepWorld")
              (Transformation|AttachComponentToComponent (Variables|Ingredient|GetCurrentIngredient) (Variables|/Game/CookingSystemComponent/Blueprints/Furnitures/BP_KitchenDesk.BP_KitchenDesk_C|GetIngredientSocket DeliveryStation) "None" "SnapToTarget" "KeepWorld" "KeepWorld" true)
              (Variables|/Game/CookingSystemComponent/Blueprints/Furnitures/BP_KitchenDesk.BP_KitchenDesk_C|SetIngredient DeliveryStation (Variables|Ingredient|GetCurrentIngredient))
              (Variables|Ingredient|SetCurrentIngredient 0)
              (if (Variables|Default|GetSimulateGame?)
                (goto _label Break))))
          (:Completed
            (CallFunction|UpdateHUD)
            (Math|Integer|IncrementInt (Variables|Orders|GetDeliveredOrders)
              (:%20%20
                (bind _asgi_game_instance (Utilities|Casting|CastToGI_GameInstance (Game|GetGameInstance)))
                (Default|UpdatePoint _asgi_game_instance (Variables|Default|GetMoney))))))
        (else
          (goto _label_2))))
    (:CastFailed
      (Utilities|Casting|CastToBP_Plate (Variables|/Game/CookingSystemComponent/Blueprints/Furnitures/BP_KitchenDesk.BP_KitchenDesk_C|GetIngredient DeliveryStation))
      ;[1 1 1] PichUpPlate
      (Utilities|IsValid (Variables|Ingredient|GetCurrentIngredient)
        (:Is%20Not%20Valid
          (Transformation|DetachFromActor (Variables|/Game/CookingSystemComponent/Blueprints/Furnitures/BP_KitchenDesk.BP_KitchenDesk_C|GetIngredient DeliveryStation) "KeepWorld" "KeepWorld" "KeepWorld")
          (Transformation|AttachComponentToComponent (Variables|/Game/CookingSystemComponent/Blueprints/Furnitures/BP_KitchenDesk.BP_KitchenDesk_C|GetIngredient DeliveryStation) (Variables|Default|GetIngredientSocket) "None" "SnapToTarget" "KeepWorld" "KeepWorld" true)
          (Variables|Ingredient|SetCurrentIngredient (Variables|/Game/CookingSystemComponent/Blueprints/Furnitures/BP_KitchenDesk.BP_KitchenDesk_C|GetIngredient DeliveryStation))
          (Variables|/Game/CookingSystemComponent/Blueprints/Furnitures/BP_KitchenDesk.BP_KitchenDesk_C|SetIngredient DeliveryStation 0))))))

(fn KitchenDeskFunction
  (params (KitchenDesk :type BP%20Kitchen%20Desk%20Object%20Reference))
  (Utilities|IsValid (Variables|/Game/CookingSystemComponent/Blueprints/Furnitures/BP_KitchenDesk.BP_KitchenDesk_C|GetIngredient KitchenDesk)
    (:Is%20Valid
      (Utilities|IsValid (Variables|Ingredient|GetCurrentIngredient)
        (:Is%20Valid
          ;[1 1 1] Combine ingredients
          (bind _asbp_ingredient (Utilities|Casting|CastToBP_Ingredient (Variables|/Game/CookingSystemComponent/Blueprints/Furnitures/BP_KitchenDesk.BP_KitchenDesk_C|GetIngredient KitchenDesk)))
          (Default|CombineIngredients _asbp_ingredient self (Variables|Ingredient|GetCurrentIngredient) KitchenDesk))
        (:Is%20Not%20Valid
          ;[1 1 1] Pick up ingredient from the kitchen desk
          (Transformation|DetachFromActor (Variables|/Game/CookingSystemComponent/Blueprints/Furnitures/BP_KitchenDesk.BP_KitchenDesk_C|GetIngredient KitchenDesk) "KeepWorld" "KeepWorld" "KeepWorld")
          (bind _output_get (Variables|Ingredient|SetCurrentIngredient (Variables|/Game/CookingSystemComponent/Blueprints/Furnitures/BP_KitchenDesk.BP_KitchenDesk_C|GetIngredient KitchenDesk)))
          (Transformation|AttachComponentToComponent _output_get (Variables|Default|GetIngredientSocket) "None" "SnapToTarget" "KeepWorld" "KeepWorld" true)
          (Variables|/Game/CookingSystemComponent/Blueprints/Furnitures/BP_KitchenDesk.BP_KitchenDesk_C|SetIngredient KitchenDesk 0))))
    (:Is%20Not%20Valid
      (Utilities|IsValid (Variables|Ingredient|GetCurrentIngredient)
        (:Is%20Valid
          ;[1 1 1] Drop on kitchen desk
          (Transformation|DetachFromActor (Variables|Ingredient|GetCurrentIngredient) "KeepWorld" "KeepWorld" "KeepWorld")
          (Transformation|AttachComponentToComponent (Variables|Ingredient|GetCurrentIngredient) (Variables|/Game/CookingSystemComponent/Blueprints/Furnitures/BP_KitchenDesk.BP_KitchenDesk_C|GetIngredientSocket KitchenDesk) "None" "SnapToTarget" "KeepWorld" "KeepWorld" true)
          (Variables|/Game/CookingSystemComponent/Blueprints/Furnitures/BP_KitchenDesk.BP_KitchenDesk_C|SetIngredient KitchenDesk (Variables|Ingredient|GetCurrentIngredient))
          (Variables|Ingredient|SetCurrentIngredient 0))))))

(fn UpdateHUD
  (bind _hudref (Variables|Default|GetHUDRef))
  (bind _orderspanel (Variables|/Game/CookingSystemComponent/Widgets/WB_HUD.WB_HUD_C|GetOrdersPanel _hudref))
  (Widget|Panel|ClearChildren _orderspanel)
  (for _array_element (Variables|Orders|GetOrders)
    (bind _returnvalue (UserInterface|CreateWidget "/Game/CookingSystemComponent/Widgets/WB_Order_Food.WB_Order_Food_C" 0 (.time _array_element) (.foodcompile _array_element)))
    (Class|HorizontalBox|AddChildtoHorizontalBox _orderspanel _returnvalue)))

(fn AddOrder
  (bind _orders (Variables|Orders|GetOrders))
  (if (<= (Utilities|Array|Length _orders) (Variables|Default|GetFatalNumber))
    (Utilities|Array|Add _orders (.OutItem (Utilities|Array|Random (Variables|Default|GetOrderAll))))
    (CallFunction|UpdateHUD)
    (else
      (Game|SetGamePaused true)
      (bind _returnvalue (UserInterface|CreateWidget "/Game/WBp/WBP_LoseGame.WBP_LoseGame_C"))
      (UserInterface|Viewport|AddtoViewport _returnvalue 0)
      (Variables|/Script/Engine.PlayerController|SetbShowMouseCursor (Game|GetPlayerController 0) true))))

(fn TrashBinFunction
  (params (TrashBin :type BP%20Trash%20Bin%20Object%20Reference))
  ;[1 1 1] Trash dish functionality
  (bind _asbp_plate (Utilities|Casting|CastToBP_Plate (Variables|Ingredient|GetCurrentIngredient))
    (:then
      (Default|Restart _asbp_plate)
      (Transformation|DetachFromActor (Variables|Ingredient|GetCurrentIngredient) "KeepWorld" "KeepWorld" "KeepWorld")
      (Transformation|AttachComponentToComponent (Variables|Ingredient|GetCurrentIngredient) (Variables|/Game/CookingSystemComponent/Blueprints/Furnitures/BP_KitchenDesk.BP_KitchenDesk_C|GetIngredientSocket TrashBin) "None" "SnapToTarget" "KeepWorld" "KeepWorld" true)
      (Variables|/Game/CookingSystemComponent/Blueprints/Furnitures/BP_KitchenDesk.BP_KitchenDesk_C|SetIngredient TrashBin (Variables|Ingredient|GetCurrentIngredient))
      (Variables|Ingredient|SetCurrentIngredient 0))
    (:CastFailed
      ;[1 1 1] PichUpPlate
      (Utilities|Casting|CastToBP_Plate (Variables|/Game/CookingSystemComponent/Blueprints/Furnitures/BP_KitchenDesk.BP_KitchenDesk_C|GetIngredient TrashBin)
        (:then
          (Utilities|IsValid (Variables|Ingredient|GetCurrentIngredient)
            (:Is%20Not%20Valid
              (Transformation|DetachFromActor (Variables|/Game/CookingSystemComponent/Blueprints/Furnitures/BP_KitchenDesk.BP_KitchenDesk_C|GetIngredient TrashBin) "KeepWorld" "KeepWorld" "KeepWorld")
              (Transformation|AttachComponentToComponent (Variables|/Game/CookingSystemComponent/Blueprints/Furnitures/BP_KitchenDesk.BP_KitchenDesk_C|GetIngredient TrashBin) (Variables|Default|GetIngredientSocket) "None" "SnapToTarget" "KeepWorld" "KeepWorld" true)
              (Variables|Ingredient|SetCurrentIngredient (Variables|/Game/CookingSystemComponent/Blueprints/Furnitures/BP_KitchenDesk.BP_KitchenDesk_C|GetIngredient TrashBin))
              (Variables|/Game/CookingSystemComponent/Blueprints/Furnitures/BP_KitchenDesk.BP_KitchenDesk_C|SetIngredient TrashBin 0))))
        (:CastFailed
          ;[1 1 1] Trash ingredient functionality
          (bind _asbp_ingredient (Utilities|Casting|CastToBP_Ingredient (Variables|Ingredient|GetCurrentIngredient)))
          (Transformation|DetachFromActor (Variables|Ingredient|GetCurrentIngredient) "KeepWorld" "KeepWorld" "KeepWorld")
          (Variables|Ingredient|SetCurrentIngredient 0)
          (Actor|DestroyActor _asbp_ingredient))))))

(fn Check
  (params (Have :type Map%20of%20BP%20Ingredient%20Class%20References%20to%20Integers) (Want :type Map%20of%20BP%20Ingredient%20Class%20References%20to%20Integers))
  (bind _keys (Utilities|Map|Keys Have))
  (for _array_element _keys
    (if (!= (.ReturnValue (Utilities|Map|Find Want _array_element)) true)
      (return false)))
  (bind _keys_2 (Utilities|Map|Keys Want))
  (for _array_element_2 _keys_2
    (if (!= (.ReturnValue (Utilities|Map|Find Have _array_element_2)) true)
      (return false)))
  (return true))