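; Player character for a cooking game, moving along fixed world axes and handling cooking input.
; Axis inputs add movement, and while held they smoothly turn the mesh toward the input direction using a shortest-path rotator lerp scaled by delta time.
; The cooking system component is initialized on BeginPlay with the player and ingredient socket, then receives the Interact and Chop presses.
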(event EventBeginPlay
  ;[1 0 0] Begin Play
  (Default|InitSystem (Variables|Default|GetBPC_CookingSystem) self (Variables|Default|GetIngredientSocket) true))

(event Input|ActionEvents|InputActionChop
  (params (Key :type Key%20Structure))
  ;[0 1 0] Chop
  (:Pressed
    (Default|ChopEvent (Variables|Default|GetBPC_CookingSystem))))

(event Input|ActionEvents|InputActionInteract
  (params (Key :type Key%20Structure))
  ;[0 0 1] Interact
  (:Pressed
    (Default|InteractEvent (Variables|Default|GetBPC_CookingSystem))))

(event Input|AxisEvents|InputAxisForwardBackward
  (params (AxisValue :type Float%20%28single-precision%29))
  ;[0.5 0.5 0.5] Movement
  (Pawn|Input|AddMovementInput "1.000000,0.000000, 0" AxisValue false)
  (if (or (!= (Input|AxisValues|GetForwardBackward) 0.0) (!= (Input|AxisValues|GetLeftRight) 0.0))
    ;;[0.5 0.5 0.5] Set desired direction
    (Variables|Movement|SetDesiredDirection (Math|Vector|MakeVector (Input|AxisValues|GetLeftRight) (* (Input|AxisValues|GetForwardBackward) -1.0) 0.0))
    (Transformation|SetWorldRotation (Variables|Character|GetMesh) (Math|Rotator|Lerp(Rotator) (Transformation|GetWorldRotation (Variables|Character|GetMesh)) (Math|Conversions|RotationFromXVector (Variables|Movement|GetDesiredDirection)) (* (Variables|Movement|GetRotationSpeed) (Utilities|Time|GetWorldDeltaSeconds)) true) false false)))

(event Input|AxisEvents|InputAxisLeftRight
  (params (AxisValue :type Float%20%28single-precision%29))
  ;[0.5 0.5 0.5] Movement
  (Pawn|Input|AddMovementInput "0.000000,1.000000, 0" AxisValue false)
  (if (or (!= (Input|AxisValues|GetForwardBackward) 0.0) (!= (Input|AxisValues|GetLeftRight) 0.0))
    ;;[0.5 0.5 0.5] Set desired direction
    (Variables|Movement|SetDesiredDirection (Math|Vector|MakeVector (Input|AxisValues|GetLeftRight) (* (Input|AxisValues|GetForwardBackward) -1.0) 0.0))
    (Transformation|SetWorldRotation (Variables|Character|GetMesh) (Math|Rotator|Lerp(Rotator) (Transformation|GetWorldRotation (Variables|Character|GetMesh)) (Math|Conversions|RotationFromXVector (Variables|Movement|GetDesiredDirection)) (* (Variables|Movement|GetRotationSpeed) (Utilities|Time|GetWorldDeltaSeconds)) true) false false)))

(fn ConstructionScript)