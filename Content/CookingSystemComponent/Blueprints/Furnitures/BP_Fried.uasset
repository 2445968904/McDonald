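; BP_Fried is a cooking furniture Blueprint that fries the ingredient it references.
; On every Tick, after the parent Tick runs, it casts its Ingredient variable to BP_Ingredient and calls Fried on it when CanBeFried is true.
; The frying behavior itself lives in BP_Ingredient, and the construction script only calls its parent.
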(event EventBeginPlay
  (|CallParentFunction) ; This node is disabled and will not be called.\nDrag off pins to build functionality.
)

(event Collision|EventActorBeginOverlap
  (params (OtherActor :type Actor%20Object%20Reference))
  (|CallParentFunction OtherActor) ; This node is disabled and will not be called.\nDrag off pins to build functionality.
)

(event EventTick
  (params (DeltaSeconds :type Float%20%28single-precision%29))
  (|CallParentFunction DeltaSeconds)
  (bind _asbp_ingredient (Utilities|Casting|CastToBP_Ingredient (Variables|Default|GetIngredient)))
  (if (Variables|/Game/CookingSystemComponent/Blueprints/Ingredients/BP_Ingredient.BP_Ingredient_C|GetCanBeFried _asbp_ingredient)
    (Default|Fried _asbp_ingredient)))

(fn ConstructionScript
  (|CallParentFunction))