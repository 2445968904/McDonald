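; BP_Ingredient is a cooking ingredient actor that turns into a chopped, grilled or fried version as it is processed.
; Each repeated processing call advances a shared Progress value by delta time and briefly shows a progress bar widget via a retriggerable delay.
; At full progress it spawns the result class, assigns it to the parent station and destroys itself.
; CombineIngredients swaps ingredients, attaching itself to the component's socket and the other to the desk.
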(event Custom|CombineIngredients
  (params (ComponentRef :type BPC%20Cooking%20System%20Object%20Reference) (SecondIngredient :type Actor%20Object%20Reference) (Desk :type BP%20Kitchen%20Desk%20Object%20Reference))
  (bind _asbp_ingredient (Utilities|Casting|CastToBP_Ingredient SecondIngredient))
  (Variables|/Game/CookingSystemComponent/Blueprints/Furnitures/BP_KitchenDesk.BP_KitchenDesk_C|SetIngredient Desk _asbp_ingredient)
  (Variables|/Game/CookingSystemComponent/Blueprints/BPC_CookingSystem.BPC_CookingSystem_C|SetCurrentIngredient ComponentRef self)
  (Transformation|AttachComponentToComponent (Variables|/Game/CookingSystemComponent/Blueprints/BPC_CookingSystem.BPC_CookingSystem_C|GetIngredientSocket ComponentRef) "None" "SnapToTarget" "KeepWorld" "KeepWorld" true)
  (Transformation|AttachComponentToComponent _asbp_ingredient (Variables|/Game/CookingSystemComponent/Blueprints/Furnitures/BP_KitchenDesk.BP_KitchenDesk_C|GetIngredientSocket Desk) "None" "SnapToTarget" "KeepWorld" "KeepWorld" true))

(event Custom|ChopIngredient
  (bind _widget (Variables|Default|GetWidget))
  (Variables|/Game/CookingSystemComponent/Widgets/WB_IngredientProgressBar.WB_IngredientProgressBar_C|SetProgress (Variables|Default|GetWB_ProgressBarRef) (Variables|Default|GetProgress))
  (if (< (Variables|Default|GetProgress) 1.0)
    (Variables|Default|SetProgress (+ (Variables|Default|GetProgress) (* (Utilities|Time|GetWorldDeltaSeconds) 0.5)))
    (Rendering|SetVisibility _widget true false)
    (Utilities|FlowControl|RetriggerableDelay 0.15)
    (Rendering|SetVisibility _widget false false)
    (else
      (bind _returnvalue (Game|SpawnActorfromClass (Variables|Default|GetChoppedIngredient) (Transformation|GetActorTransform) "Undefined" 0 0))
      (bind _asbp_chopping_table (Utilities|Casting|CastToBP_ChoppingTable (Actor|GetAttachParentActor)))
      (Variables|/Game/CookingSystemComponent/Blueprints/Furnitures/BP_KitchenDesk.BP_KitchenDesk_C|SetIngredient _asbp_chopping_table _returnvalue)
      (Actor|DestroyActor))))

(event Custom|Fried
  (bind _widget (Variables|Default|GetWidget))
  (Variables|/Game/CookingSystemComponent/Widgets/WB_IngredientProgressBar.WB_IngredientProgressBar_C|SetProgress (Variables|Default|GetWB_ProgressBarRef) (Variables|Default|GetProgress))
  (if (< (Variables|Default|GetProgress) 1.0)
    (Variables|Default|SetProgress (+ (Variables|Default|GetProgress) (* (Utilities|Time|GetWorldDeltaSeconds) 0.5)))
    (Rendering|SetVisibility _widget true false)
    (Utilities|FlowControl|RetriggerableDelay 0.15)
    (Rendering|SetVisibility _widget false false)
    (else
      (bind _returnvalue (Game|SpawnActorfromClass (Variables|Default|GetFriedIngredient) (Transformation|GetActorTransform) "Undefined" 0 0))
      (bind _asbp_fried (Utilities|Casting|CastToBP_Fried (Actor|GetAttachParentActor)))
      (Variables|/Game/CookingSystemComponent/Blueprints/Furnitures/BP_KitchenDesk.BP_KitchenDesk_C|SetIngredient _asbp_fried _returnvalue)
      (Actor|DestroyActor))))

(event Custom|GrillIngredient
  (bind _widget (Variables|Default|GetWidget))
  (Variables|/Game/CookingSystemComponent/Widgets/WB_IngredientProgressBar.WB_IngredientProgressBar_C|SetProgress (Variables|Default|GetWB_ProgressBarRef) (Variables|Default|GetProgress))
  (if (< (Variables|Default|GetProgress) 1.0)
    (Variables|Default|SetProgress (+ (Variables|Default|GetProgress) (* (Utilities|Time|GetWorldDeltaSeconds) 0.5)))
    (Rendering|SetVisibility _widget true false)
    (Utilities|FlowControl|RetriggerableDelay 0.15)
    (Rendering|SetVisibility _widget false false)
    (else
      (bind _returnvalue (Game|SpawnActorfromClass (Variables|Default|GetGrilledIngredient) (Transformation|GetActorTransform) "Undefined" 0 0))
      (bind _asbp_grill (Utilities|Casting|CastToBP_Grill (Actor|GetAttachParentActor)))
      (Variables|/Game/CookingSystemComponent/Blueprints/Furnitures/BP_KitchenDesk.BP_KitchenDesk_C|SetIngredient _asbp_grill _returnvalue)
      (Actor|DestroyActor))))

(event EventBeginPlay
  (bind _aswb_ingredient_progress_bar (Utilities|Casting|CastToWB_IngredientProgressBar (UserInterface|GetUserWidgetObject (Variables|Default|GetWidget))))
  (Variables|Default|SetWB_ProgressBarRef _aswb_ingredient_progress_bar))

(fn ConstructionScript)