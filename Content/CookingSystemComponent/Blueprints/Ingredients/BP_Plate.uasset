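; Plate for the cooking system that collects ingredients flagged CanOnPlate, one of each class, as a dish is assembled.
; CombineIngredients records the class in NowHaveFood, copies the ingredient's mesh into a runtime component, then destroys the ingredient.
; Restart clears that map, resets dish state and hides cached meshes without destroying them.
; An older hardcoded burger/salad path, the only caller of SetDish, remains as unreachable nodes.
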(event EventBeginPlay
  (|CallParentFunction) ; This node is disabled and will not be called.\nDrag off pins to build functionality.
)

(event Collision|EventActorBeginOverlap
  (params (OtherActor :type Actor%20Object%20Reference)))

(event EventTick
  (params (DeltaSeconds :type Float%20%28single-precision%29)))

(event EventCombineIngredients
  (params (ComponentRef :type BPC%20Cooking%20System%20Object%20Reference) (SecondIngredient :type Actor%20Object%20Reference) (Desk :type BP%20Kitchen%20Desk%20Object%20Reference))
  (bind _asbp_ingredient (Utilities|Casting|CastToBP_Ingredient SecondIngredient))
  (if (Variables|/Game/CookingSystemComponent/Blueprints/Ingredients/BP_Ingredient.BP_Ingredient_C|GetCanOnPlate _asbp_ingredient)
    (if (not (.ReturnValue (Utilities|Map|Find (Variables|Default|GetNowHaveFood) (Utilities|GetClass _asbp_ingredient))))
      (Utilities|Map|Add (Variables|Default|GetNowHaveFood) (Utilities|GetClass _asbp_ingredient) 1)
      (bind _returnvalue (AddComponent|AddStaticMeshComponent false))
      (Components|StaticMesh|SetStaticMesh _returnvalue (Variables|/Script/Engine.StaticMeshComponent|GetStaticMesh (Actor|GetComponentbyClass SecondIngredient "/Script/Engine.StaticMeshComponent")))
      (Actor|DestroyActor SecondIngredient)
      (Variables|/Game/CookingSystemComponent/Blueprints/BPC_CookingSystem.BPC_CookingSystem_C|SetCurrentIngredient ComponentRef 0)
      (Utilities|Array|Add (Variables|Default|GetStaticMeshCache) _returnvalue))
    (else
      (Utilities|Casting|CastToBP_Plate SecondIngredient)
      (|CallParentFunction ComponentRef SecondIngredient Desk))))

(fn ConstructionScript
  (|CallParentFunction))

(fn SetDish
  (if (Math|Boolean|ANDBoolean (Variables|Default|GetHasBun?) (Variables|Default|GetHasMeat?) (Variables|Default|GetHasLettuce?) (Variables|Default|GetHasTomato?))
    (Variables|Default|SetDish "NewEnumerator0")
    (elif (and (Variables|Default|GetHasLettuce?) (Variables|Default|GetHasLettuce?))
      (Variables|Default|SetDish "NewEnumerator1"))))

(fn Restart
  (Utilities|FlowControl|Sequence
    (:then_0
      (Variables|Default|SetHasLettuce? false)
      (Variables|Default|SetHasTomato? false)
      (Variables|Default|SetHasMeat? false)
      (Variables|Default|SetHasBun? false)
      (Variables|Default|SetDish "NewEnumerator4"))
    (:then_1
      (Utilities|Map|Clear (Variables|Default|GetNowHaveFood)))
    (:then_2
      (for _array_element (Variables|Default|GetStaticMeshCache)
        (Rendering|SetVisibility _array_element false false)))))